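; Pinball game mode Blueprint that handles scoring and ball loss.
; AddScore casts to bp_pinballgamestate and adds the given points to its stored score.
; OnBallLost decrements the game state's remaining balls, then calls SpawnBall while any remain, otherwise only prints "Game Over".
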(event EventBeginPlay
  (|CallParentFunction))

(event EventTick
  (params (DeltaSeconds :type Float%20%28single-precision%29))
  (|CallParentFunction DeltaSeconds) ; This node is disabled and will not be called.\nDrag off pins to build functionality.
)

(event EventAddScore
  (params (points :type Float%20%28double-precision%29))
  (bind _asbp_pinballgamestate (Utilities|Casting|CastTobp_pinballgamestate (Game|GetGameState)))
  (Default|SetScore _asbp_pinballgamestate (+ points (Variables|/Game/bp_pinballgamestate.bp_pinballgamestate_C|Getscore _asbp_pinballgamestate))))

(event EventOnBallLost
  (bind _asbp_pinballgamestate (Utilities|Casting|CastTobp_pinballgamestate (Game|GetGameState)))
  (bind _result (Math|Integer|DecrementInt (Variables|/Game/bp_pinballgamestate.bp_pinballgamestate_C|Getballs_remaining _asbp_pinballgamestate))
    (:%20%20
      (Default|SetBalls _asbp_pinballgamestate _result)
      (if (> _result 0)
        (CallFunction|SpawnBall)
        (else
          (Development|PrintString "Game Over"))))))

(fn ConstructionScript
  (|CallParentFunction))