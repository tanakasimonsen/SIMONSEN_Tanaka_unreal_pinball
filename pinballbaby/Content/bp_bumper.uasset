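; Pinball pop bumper actor that knocks reactive objects away and awards points when they touch it.
; On capsule overlap it sends a max-force impulse, directed away from the bumper's center, through the pinball-reactive interface, then adds score via the game mode's score-receiver interface.
; A timeline lerps the bumper mechanism mesh between start and end positions; ending the overlap stops it and snaps the mesh back.
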(event OnComponentBeginOverlap(Capsule)
  (params (OverlappedComponent :type Primitive%20Component%20Object%20Reference) (OtherActor :type Actor%20Object%20Reference) (OtherComp :type Primitive%20Component%20Object%20Reference) (OtherBodyIndex :type Integer) (bFromSweep :type Boolean) (SweepResult :type Hit%20Result%20Structure%20%28by%20ref%29))
  (Utilities|FlowControl|Sequence
    (:then_0
      ;[0.15 0.15 0.15 0.5] apply pinball force
      (bind _asbpi_pinballreactive (Utilities|Casting|CastTobpi_pinballreactive OtherActor)
        (:then
          (Default|PinballImpulseEvent _asbpi_pinballreactive (* (Variables|Default|Getmax_force) (Math|Vector|Normalize (- (Transformation|GetWorldLocation OtherComp) (Transformation|GetActorLocation)))))
          (bind _asbpi_scorereceiver (Utilities|Casting|CastTobpi_scorereceiver (Game|GetGameMode)))
          (Default|AddScore _asbpi_scorereceiver (Variables|Default|Getscore_value)))
        (:CastFailed
          (Development|PrintString "failed here"))))
    (:then_1
      ;[0.15 0.15 0.15 0.5] play animation
      (bind _newtrack_0 (Timeline|Timeline PlayFromStart)
        (:Update
          (Transformation|SetRelativeLocation (Variables|Default|GetSM_PopBumperMechanism) (Math|Vector|Lerp(Vector) (Variables|Default|Getstart_pos) (Variables|Default|Getend_pos) _newtrack_0) false false))))))

(event OnComponentEndOverlap(Capsule)
  (params (OverlappedComponent :type Primitive%20Component%20Object%20Reference) (OtherActor :type Actor%20Object%20Reference) (OtherComp :type Primitive%20Component%20Object%20Reference) (OtherBodyIndex :type Integer))
  (Utilities|FlowControl|Sequence
    (:then_0
      ;[0.15 0.15 0.15 0.5] play animation
      (bind _newtrack_0 (Timeline|Timeline Stop)
        (:Update
          (Transformation|SetRelativeLocation (Variables|Default|GetSM_PopBumperMechanism) (Math|Vector|Lerp(Vector) (Variables|Default|Getstart_pos) (Variables|Default|Getend_pos) _newtrack_0) false false))))
    (:then_1
      (Transformation|SetRelativeLocation (Variables|Default|GetSM_PopBumperMechanism) (Variables|Default|Getstart_pos) false false))))

(event EventBeginPlay)

(event Collision|EventActorBeginOverlap
  (params (OtherActor :type Actor%20Object%20Reference)))

(event EventTick
  (params (DeltaSeconds :type Float%20%28single-precision%29)))

(fn ConstructionScript)