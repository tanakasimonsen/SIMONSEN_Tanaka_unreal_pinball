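; Flipper actor, likely for pinball, that swings between resting and flipped rotations when activated and deactivated.
; A Direction enum orients the pivot in the construction script and selects the sign of the quarter-turn swing, computed at BeginPlay.
; The activate event plays a timeline that lerps the flipper's relative rotation between the two poses.
; The deactivate event reverses that timeline to return it to rest.
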(event Custom|OnActivate_Event
  ;[0.15 0.15 0.15 0.5] Flipper Movement
  (bind _newtrack_0 (Timeline|0-1 Play)
    (:Update
      (Transformation|SetRelativeRotation (Variables|Default|Getflipper) (Math|Rotator|Lerp(Rotator) (Variables|Default|Getflipper_resting) (Variables|Default|Getflipper_flipped) _newtrack_0) false false))))

(event Custom|OnDeactivate_Event
  ;[0.15 0.15 0.15 0.5] Flipper Movement
  (bind _newtrack_0 (Timeline|0-1 Reverse)
    (:Update
      (Transformation|SetRelativeRotation (Variables|Default|Getflipper) (Math|Rotator|Lerp(Rotator) (Variables|Default|Getflipper_resting) (Variables|Default|Getflipper_flipped) _newtrack_0) false false))))

(event Collision|EventActorBeginOverlap
  (params (OtherActor :type Actor%20Object%20Reference)))

(event EventBeginPlay
  ;[0.15 0.15 0.15 0.5] Setup
  (bind _output_get (Variables|Default|Setflipper_resting "0, 0, 0"))
  (Variables|Default|Setflipper_flipped (Math|Rotator|CombineRotators _output_get (Math|Rotator|SelectRotator "0.000000,-90.000000,0.000000" "0.000000,90.000000,0.000000" (Utilities|Enum|Equal(Enum) (Variables|Default|Getdirection) "NewEnumerator0")))))

(fn ConstructionScript
  (Transformation|SetRelativeRotation (Variables|Default|Getflipper_pivot) (Math|Rotator|SelectRotator "0.000000,180.000000,0.000000" "0, 0, 0" (Utilities|Enum|Equal(Enum) (Variables|Default|Getdirection) "NewEnumerator0")) false false))