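; Pinball plunger Blueprint that animates a plunger mesh pulling back and releasing through charge and release events.
; A charge timeline lerps the mesh from start to end position while recording charge time and current position.
; Release stops that timeline and a second one lerps the mesh back to start.
; The box end-overlap casts to the pinball-reactive type, but the charge-scaled impulse call is unconnected, so no launch force is applied.
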(event OnComponentEndOverlap(Box)
  (params (OverlappedComponent :type Primitive%20Component%20Object%20Reference) (OtherActor :type Actor%20Object%20Reference) (OtherComp :type Primitive%20Component%20Object%20Reference) (OtherBodyIndex :type Integer))
  (bind _asbpi_pinballreactive (Utilities|Casting|CastTobpi_pinballreactive OtherActor)))

(event Custom|plunger_charge_Event
  ;[0.15 0.15 0.15 0.5] charge time
  (bind _0_1 (Timeline|Timeline PlayFromStart)
    (:Update
      (Variables|Default|Setcharge_time _0_1)
      (Variables|Default|Setupdated_pos (Math|Vector|Lerp(Vector) (Variables|Default|Getstart_pos) (Variables|Default|Getend_pos) _0_1))
      (Transformation|SetRelativeLocation (Variables|Default|GetSM_Plunger) (Math|Vector|Lerp(Vector) (Variables|Default|Getstart_pos) (Variables|Default|Getend_pos) _0_1) false false))))

(event Custom|plunger_release_Event
  ;[0.15 0.15 0.15 0.5] plunger release
  (Utilities|FlowControl|Sequence
    (:then_0
      ;[0.15 0.15 0.15 0.5] charge time
      (bind _0_1 (Timeline|Timeline Stop)
        (:Update
          (Variables|Default|Setcharge_time _0_1)
          (Variables|Default|Setupdated_pos (Math|Vector|Lerp(Vector) (Variables|Default|Getstart_pos) (Variables|Default|Getend_pos) _0_1))
          (Transformation|SetRelativeLocation (Variables|Default|GetSM_Plunger) (Math|Vector|Lerp(Vector) (Variables|Default|Getstart_pos) (Variables|Default|Getend_pos) _0_1) false false))))
    (:then_1
      (bind _0_1_2 (Timeline|Timeline_0 PlayFromStart)
        (:Update
          (Transformation|SetRelativeLocation (Variables|Default|GetSM_Plunger) (Math|Vector|Lerp(Vector) (Variables|Default|Getupdated_pos) (Variables|Default|Getstart_pos) _0_1_2) false false))))))

(event EventBeginPlay)

(event Collision|EventActorBeginOverlap
  (params (OtherActor :type Actor%20Object%20Reference)))

(event EventTick
  (params (DeltaSeconds :type Float%20%28single-precision%29)))

(fn ConstructionScript)