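; Pinball game state Blueprint that tracks the score and the number of balls remaining.
; On BeginPlay it seeds both values through its setter events.
; Each setter stores the new value, calls a matching changed dispatcher so other objects can react, and prints the value for debugging.
; Tick and the construction script are empty.
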(event Custom|set_score
  (params (new_score :type Float%20%28double-precision%29))
  (bind _output_get (Variables|Default|Setscore new_score))
  (Default|CallOnScoreChanged _output_get)
  (Development|PrintString (Utilities|String|ToString(Float) _output_get)))

(event Custom|set_balls
  (params (new_balls :type Integer))
  (bind _output_get (Variables|Default|Setballs_remaining new_balls))
  (Default|CallOnBallsChanged _output_get)
  (Development|PrintString (Utilities|String|ToString(Integer) _output_get)))

(event EventBeginPlay
  (CallFunction|SetScore 1e+02)
  (CallFunction|SetBalls 3))

(event EventTick
  (params (DeltaSeconds :type Float%20%28single-precision%29)))

(fn ConstructionScript)